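; A small diagonal-moving enemy for a space shooter minigame.
; Tick moves it along local Y while bouncing it horizontally between fixed X limits with swept offsets.
; Overlapping any of four player projectile classes destroys both actors and sends score to the HUD; a shield overlap only sends score.
; A separate Destroy event plays explosion effects and sound before removing the enemy.
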(event `self.ReceiveTick`
  (params (DeltaSeconds :type "Float (single-precision)"))
  (bind _x (.x (`self.K2_GetActorLocation`)))
  (if (>= _x 270.0)
    (set `self.HorzMovementDirection` -1.0)
    (elif (<= _x -270.0)
      (set `self.HorzMovementDirection` 1.0)))
  (`self.K2_AddActorLocalOffset` (`KismetMathLibrary.MakeVector` (* DeltaSeconds (* (`self.HorzMovementSpeed`) (`self.HorzMovementDirection`))) (* DeltaSeconds (`self.Speed`))) true))

(event `self.ReceiveActorBeginOverlap`
  (params (OtherActor :type "Actor Object Reference"))
  (bind _returnvalue (`GameplayStatics.GetObjectClass` OtherActor))
  (if (== _returnvalue "/Game/Blueprints/GAB_SpaceShooterPlayerProj01.GAB_SpaceShooterPlayerProj01_C")
    (`self.K2_DestroyActor` OtherActor :!label _label)
    (`self.K2_DestroyActor`)
    (message `/Game/Blueprints/GAB_SpaceShooterBlueprintInterfacesBlue.EnemyDestroyedUpdateScore` (`PlayerController.GetHUD` (`GameplayStatics.GetPlayerController` 0)) 150 :!label _label_2)
    (elif (== _returnvalue "/Game/Blueprints/GAB_SpaceShooterPlayerProj02.GAB_SpaceShooterPlayerProj02_C")
      (goto _label)
      (elif (== _returnvalue "/Game/Blueprints/GAB_SpaceShooterPlayerProj03.GAB_SpaceShooterPlayerProj03_C")
        (goto _label)
        (elif (== _returnvalue "/Game/Blueprints/GAB_SpaceShooterPlayerProj04.GAB_SpaceShooterPlayerProj04_C")
          (goto _label)
          (elif (== _returnvalue "/Game/Blueprints/GAB_SpaceShooterShield.GAB_SpaceShooterShield_C")
            (goto _label_2)))))))

(event `Destroy`
  (`GameplayStatics.SpawnEmitterAtLocation` "/Game/Particles/P_Explosion.P_Explosion" (`self.K2_GetActorLocation`))
  (`GameplayStatics.PlaySoundAtLocation` "/Game/ImportedSounds/Retard_alvert.Retard_alvert" (0.0 0.0 0.0) (struct) 1.0 1.0 0.0 null null null)
  (`self.K2_DestroyActor`))

(fn `UserConstructionScript`
  (`parent.UserConstructionScript`))