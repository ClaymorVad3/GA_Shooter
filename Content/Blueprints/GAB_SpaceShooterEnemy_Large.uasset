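; Large enemy ship for a space shooter that drifts steadily along its local negative Y axis with a swept move.
; After a random start delay, it fires large enemy projectiles on a repeating timer.
; Overlapping player projectiles are destroyed and drain Health; a hit at zero Health, or any shield contact, explodes it and awards score through the HUD.
; A separate Destroy event explodes it without awarding score.
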(event `self.ReceiveBeginPlay`
  (`KismetSystemLibrary.Delay` (`KismetMathLibrary.RandomFloatInRange` 0.0 1.0))
  (`|SpawnActorFromClass` "/Game/Blueprints/GAB_SpaceShooterEnemyLargeProj.GAB_SpaceShooterEnemyLargeProj_C" (`self.GetTransform`) "AdjustIfPossibleButDontSpawnIfColliding" "OverrideRootScale" null null :!label _label)
  (`GameplayStatics.PlaySoundAtLocation` "/Game/ImportedSounds/censor-beep-1.censor-beep-1" (0.0 0.0 0.0) (struct) 1.0 1.0 0.0 null null null)
  (`KismetSystemLibrary.Delay` 1.5)
  (goto _label))

(event `self.ReceiveTick`
  (params (DeltaSeconds :type "Float (single-precision)"))
  (`self.K2_AddActorLocalOffset` (`KismetMathLibrary.MakeVector` 0.0 (* DeltaSeconds -35.0)) true))

(event `self.ReceiveActorBeginOverlap`
  (params (OtherActor :type "Actor Object Reference"))
  (bind _returnvalue (`GameplayStatics.GetObjectClass` OtherActor))
  (if (== _returnvalue "/Game/Blueprints/GAB_SpaceShooterPlayerProj01.GAB_SpaceShooterPlayerProj01_C")
    (`self.K2_DestroyActor` OtherActor :!label _label_2)
    (if (> (`self.Health`) 0)
      (set `self.Health` (- (`self.Health`) 1))
      (`GameplayStatics.PlaySoundAtLocation` "/Game/Audio/Sounds/EnemyLargeImpact.EnemyLargeImpact" (0.0 0.0 0.0) (struct) 1.0 1.0 0.0 null null null)
      (else
        (`GameplayStatics.SpawnEmitterAtLocation` "/Game/Particles/P_Explosion.P_Explosion" (`self.K2_GetActorLocation`) :!label _label_3)
        (`GameplayStatics.PlaySoundAtLocation` "/Game/ImportedSounds/chewbacca_swf.chewbacca_swf" (0.0 0.0 0.0) (struct) 1.0 1.0 0.0 null null null)
        (`self.K2_DestroyActor`)
        (message `/Game/Blueprints/GAB_SpaceShooterBlueprintInterfacesBlue.EnemyDestroyedUpdateScore` (`PlayerController.GetHUD` (`GameplayStatics.GetPlayerController` 0)) 250)))
    (elif (== _returnvalue "/Game/Blueprints/GAB_SpaceShooterPlayerProj02.GAB_SpaceShooterPlayerProj02_C")
      (goto _label_2)
      (elif (== _returnvalue "/Game/Blueprints/GAB_SpaceShooterPlayerProj03.GAB_SpaceShooterPlayerProj03_C")
        (goto _label_2)
        (elif (== _returnvalue "/Game/Blueprints/GAB_SpaceShooterPlayerProj04.GAB_SpaceShooterPlayerProj04_C")
          (goto _label_2)
          (elif (== _returnvalue "/Game/Blueprints/GAB_SpaceShooterShield.GAB_SpaceShooterShield_C")
            (goto _label_3)))))))

(event `Destroy`
  (`GameplayStatics.SpawnEmitterAtLocation` "/Game/Particles/P_Explosion.P_Explosion" (`self.K2_GetActorLocation`))
  (`GameplayStatics.PlaySoundAtLocation` "/Game/ImportedSounds/shooting.shooting" (0.0 0.0 0.0) (struct) 1.0 1.0 0.0 null null null)
  (`self.K2_DestroyActor`))

(fn `UserConstructionScript`)