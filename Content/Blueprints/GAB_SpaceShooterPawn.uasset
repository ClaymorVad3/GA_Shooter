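; Player ship pawn for a space shooter, steered with WASD and firing on Space.
; Tick moves it with a swept offset and stops it at bounds measured from the camera.
; Held fire loops through delays over four weapon types, with ammo pickups switching weapons and empty ammo reverting to default.
; Body overlaps sort actors by class for damage and pickups; death triggers an explosion, then a blinking respawn with collision off.
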(event `self.ReceiveTick`
  (params (DeltaSeconds :type "Float (single-precision)"))
  (`self.K2_AddActorLocalOffset` (`KismetMathLibrary.MakeVector` (`self.CurrentSideSpeed`) (* DeltaSeconds (`self.CurrentSpeed`))) true)
  (set `self.YDistPlayerCamera` (- (.y (`self.K2_GetActorLocation` (`GameplayStatics.GetPlayerCameraManager` 0))) (.y (`self.K2_GetActorLocation`))))
  (set `self.XDistPlayerCamera` (- (.x (`self.K2_GetActorLocation` (`GameplayStatics.GetPlayerCameraManager` 0))) (.x (`self.K2_GetActorLocation`))))
  (set `self.AllowForMovement` (>= (`self.YDistPlayerCamera`) -300.0))
  (if (not (`self.AllowForMovement`))
    (set `self.CurrentSpeed` (`self.MinSpeed`)))
  (set `self.AllowBackmovement` (<= (`self.YDistPlayerCamera`) 300.0))
  (if (not (`self.AllowBackmovement`))
    (set `self.CurrentSpeed` (`self.MinSpeed`)))
  (set `self.AllowLeftMovement` (>= (`self.XDistPlayerCamera`) -275.0))
  (if (not (`self.AllowLeftMovement`))
    (set `self.CurrentSideSpeed` 0.0))
  (set `self.AllowRightMovement` (<= (`self.XDistPlayerCamera`) 275.0))
  (if (not (`self.AllowRightMovement`))
    (set `self.CurrentSideSpeed` 0.0)))

(event `Key|W` :consume false
  (params (Key :type "Key Structure"))
  (:`Pressed`
    (if (`self.AllowForMovement`)
      (set `self.CurrentSpeed` (`self.MaxSpeed`))
      (else
        (set `self.CurrentSpeed` (`self.MinSpeed`) :!label _label))))
  (:`Released`
    (goto _label)))

(event `Key|S` :consume false
  (params (Key :type "Key Structure"))
  (:`Pressed`
    (if (`self.AllowBackmovement`)
      (set `self.CurrentSpeed` (* (`self.MaxSpeed`) -1.0))
      (else
        (set `self.CurrentSpeed` (`self.MinSpeed`) :!label _label_2))))
  (:`Released`
    (goto _label_2)))

(event `self.BodyMesh.OnComponentBeginOverlap`
  (params (OverlappedComponent :type "PrimitiveComponent Object Reference") (OtherActor :type "Actor Object Reference") (OtherComp :type "PrimitiveComponent Object Reference") (OtherBodyIndex :type Integer) (bFromSweep :type Boolean) (SweepResult :type "HitResult Structure (by ref)"))
  (bind _returnvalue (`GameplayStatics.GetObjectClass` OtherActor))
  ;[1 1 1] Overlap Logic
  (if (!= _returnvalue "/Game/Blueprints/GAB_SpaceShooterShieldPickup.GAB_SpaceShooterShieldPickup_C")
    (if (!= _returnvalue "/Game/Blueprints/GAB_SpaceShooterShield.GAB_SpaceShooterShield_C")
      (if (!= _returnvalue "/Game/Blueprints/GAB_SpaceShooterPlayerProj01.GAB_SpaceShooterPlayerProj01_C")
        (if (!= _returnvalue "/Game/Blueprints/GAB_SpaceShooterPlayerProj02.GAB_SpaceShooterPlayerProj02_C")
          (if (!= _returnvalue "/Game/Blueprints/GAB_SpaceShooterPlayerProj03.GAB_SpaceShooterPlayerProj03_C")
            (if (!= _returnvalue "/Game/Blueprints/GAB_SpaceShooterPlayerProj04.GAB_SpaceShooterPlayerProj04_C")
              (if (`KismetMathLibrary.ClassIsChildOf` _returnvalue "/Game/Blueprints/GAB_SpaceShooterEnemyProj.GAB_SpaceShooterEnemyProj_C")
                (`self.K2_DestroyActor` OtherActor)
                (set `self.Health` (- (`self.Health`) 2) :!label _label_3)
                (`GameplayStatics.PlaySoundAtLocation` "/Game/ImportedSounds/the-simpsons-nelsons-haha.the-simpsons-nelsons-haha" (0.0 0.0 0.0) (struct) 1.0 1.0 0.0 null null null :!label _label_4)
                (if (<= (`self.Health`) 0)
                  (set `self.AllowForMovement` false)
                  (set `self.AllowBackmovement` false)
                  (set `self.AllowLeftMovement` false)
                  (set `self.AllowRightMovement` false)
                  (set `self.AllowFiring` false)
                  (set `self.Firing` false)
                  (`self.SetActorHiddenInGame` true)
                  (`self.SetActorEnableCollision` false)
                  (`GameplayStatics.SpawnEmitterAtLocation` "/Game/Particles/P_Explosion.P_Explosion" (`self.K2_GetActorLocation`))
                  (`GameplayStatics.PlaySoundAtLocation` null (0.0 0.0 0.0) (struct) 1.0 1.0 0.0 null null null)
                  (`KismetSystemLibrary.Delay` 2.0)
                  (set `self.Health` 100)
                  (set `self.AllowForMovement` true)
                  (set `self.AllowBackmovement` true)
                  (set `self.AllowLeftMovement` true)
                  (set `self.AllowRightMovement` true)
                  (set `self.AllowFiring` true)
                  (`self.SetActorHiddenInGame` false)
                  (`KismetSystemLibrary.Delay` 0.25)
                  (`self.SetActorHiddenInGame` true)
                  (`KismetSystemLibrary.Delay` 0.25)
                  (`self.SetActorHiddenInGame` false)
                  (`KismetSystemLibrary.Delay` 0.25)
                  (`self.SetActorHiddenInGame` true)
                  (`KismetSystemLibrary.Delay` 0.25)
                  (`self.SetActorHiddenInGame` false)
                  (`KismetSystemLibrary.Delay` 0.25)
                  (`self.SetActorHiddenInGame` true)
                  (`KismetSystemLibrary.Delay` 0.25)
                  (`self.SetActorHiddenInGame` false)
                  (`self.SetActorEnableCollision` true))
                (elif (== _returnvalue "/Game/Blueprints/GAB_SpaceShooterEnemy_SmallDiagonal01.GAB_SpaceShooterEnemy_SmallDiagonal01_C")
                  (bind _asgab_space_shooter_enemy_small_diagonal_01 (cast `/Game/Blueprints/GAB_SpaceShooterEnemy_SmallDiagonal01` OtherActor))
                  (`/Game/Blueprints/GAB_SpaceShooterEnemy_SmallDiagonal01.Destroy` _asgab_space_shooter_enemy_small_diagonal_01)
                  (goto _label_3)
                  (elif (== _returnvalue "/Game/Blueprints/GAB_SpaceShooterEnemy_SmallDiagonal02.GAB_SpaceShooterEnemy_SmallDiagonal02_C")
                    (bind _asgab_space_shooter_enemy_small_diagonal_02 (cast `/Game/Blueprints/GAB_SpaceShooterEnemy_SmallDiagonal02` OtherActor))
                    (`/Game/Blueprints/GAB_SpaceShooterEnemy_SmallDiagonal02.Destroy` _asgab_space_shooter_enemy_small_diagonal_02)
                    (goto _label_3)
                    (elif (== _returnvalue "/Game/Blueprints/GAB_SpaceShooterEnemy_SmallRandom.GAB_SpaceShooterEnemy_SmallRandom_C")
                      (bind _asgab_space_shooter_enemy_small_random (cast `/Game/Blueprints/GAB_SpaceShooterEnemy_SmallRandom` OtherActor))
                      (`/Game/Blueprints/GAB_SpaceShooterEnemy_SmallRandom.Destroy` _asgab_space_shooter_enemy_small_random)
                      (goto _label_3)
                      (elif (== _returnvalue "/Game/Blueprints/GAB_SpaceShooterEnemy_SmallStraight.GAB_SpaceShooterEnemy_SmallStraight_C")
                        (bind _asgab_space_shooter_enemy_small_straight (cast `/Game/Blueprints/GAB_SpaceShooterEnemy_SmallStraight` OtherActor))
                        (`/Game/Blueprints/GAB_SpaceShooterEnemy_SmallStraight.Destroy` _asgab_space_shooter_enemy_small_straight)
                        (goto _label_3)
                        (elif (== _returnvalue "/Game/Blueprints/GAB_SpaceShooterEnemyLargeProj.GAB_SpaceShooterEnemyLargeProj_C")
                          (`self.K2_DestroyActor` OtherActor)
                          (set `self.Health` (- (`self.Health`) 10) :!label _label_5)
                          (goto _label_4)
                          (elif (== _returnvalue "/Game/Blueprints/GAB_SpaceShooterEnemy_Large.GAB_SpaceShooterEnemy_Large_C")
                            (bind _asgab_space_shooter_enemy_large (cast `/Game/Blueprints/GAB_SpaceShooterEnemy_Large` OtherActor))
                            (`/Game/Blueprints/GAB_SpaceShooterEnemy_Large.Destroy` _asgab_space_shooter_enemy_large)
                            (goto _label_5)
                            (elif (== _returnvalue "/Game/Blueprints/GAB_SpaceShooterTurretProj.GAB_SpaceShooterTurretProj_C")
                              (`self.K2_DestroyActor` OtherActor)
                              (set `self.Health` (- (`self.Health`) 5))
                              (goto _label_4)
                              (elif (== _returnvalue "/Game/Blueprints/GAB_SpaceShooterTurret.GAB_SpaceShooterTurret_C")
                                (cast `/Game/Blueprints/GAB_SpaceShooterTurret` OtherActor)
                                (elif (== _returnvalue "/Game/Blueprints/GAB_SpaceShooterAmmo01.GAB_SpaceShooterAmmo01_C")
                                  (set `self.WeaponType` 1)
                                  (set `self.AmmoCount` 100)
                                  (`self.K2_DestroyActor` OtherActor)
                                  (elif (== _returnvalue "/Game/Blueprints/GAB_SpaceShooterAmmo02.GAB_SpaceShooterAmmo02_C")
                                    (set `self.WeaponType` 2)
                                    (set `self.AmmoCount` 100)
                                    (`self.K2_DestroyActor` OtherActor)
                                    (elif (== _returnvalue "/Game/Blueprints/GAB_SpaceShooterAmmo03.GAB_SpaceShooterAmmo03_C")
                                      (set `self.WeaponType` 3)
                                      (set `self.AmmoCount` 100)
                                      (`self.K2_DestroyActor` OtherActor)
                                      (elif (== _returnvalue "/Game/Blueprints/GAB_SpaceShooterHealth.GAB_SpaceShooterHealth_C")
                                        (set `self.Health` 100)
                                        (`self.K2_DestroyActor` OtherActor)))))))))))))))))))))

(event `Key|A` :consume false
  (params (Key :type "Key Structure"))
  (:`Pressed`
    (if (`self.AllowLeftMovement`)
      (set `self.CurrentSideSpeed` (`self.MaxSideSPeed`))
      (else
        (set `self.CurrentSideSpeed` 0.0 :!label _label_6))))
  (:`Released`
    (goto _label_6)))

(event `Key|D` :consume false
  (params (Key :type "Key Structure"))
  (:`Pressed`
    (if (`self.AllowRightMovement`)
      (set `self.CurrentSideSpeed` (* (`self.MaxSideSPeed`) -1.0))
      (else
        (set `self.CurrentSideSpeed` 0.0 :!label _label_7))))
  (:`Released`
    (goto _label_7)))

(event `Key|SpaceBar` :consume false
  (params (Key :type "Key Structure"))
  (:`Pressed`
    ;[1 1 1] Firing Logic
    (set `self.Firing` true)
    (if (`self.AllowFiring`)
      (if (`self.Firing`) :!label _label_8
        (switch `int` (`self.WeaponType`)
          (:`0`
            (`|SpawnActorFromClass` "/Game/Blueprints/GAB_SpaceShooterPlayerProj01.GAB_SpaceShooterPlayerProj01_C" (`self.GetTransform`) "AdjustIfPossibleButDontSpawnIfColliding" "OverrideRootScale" null null)
            (`GameplayStatics.PlaySoundAtLocation` "/Game/ImportedSounds/Woooow.Woooow" (0.0 0.0 0.0) (struct) 1.0 1.0 0.0 null null null)
            (`KismetSystemLibrary.Delay` 0.25)
            (goto _label_8))
          (:`1`
            (`|SpawnActorFromClass` "/Game/Blueprints/GAB_SpaceShooterPlayerProj02.GAB_SpaceShooterPlayerProj02_C" (`self.GetTransform`) "AdjustIfPossibleButDontSpawnIfColliding" "OverrideRootScale" null null)
            (`GameplayStatics.PlaySoundAtLocation` "/Game/ImportedSounds/taco-bell-bong-sfx.taco-bell-bong-sfx" (0.0 0.0 0.0) (struct) 1.0 1.0 0.0 null null null)
            (`KismetSystemLibrary.Delay` 0.15)
            (set `self.AmmoCount` (- (`self.AmmoCount`) 2))
            (if (> (`self.AmmoCount`) 0)
              (goto _label_8)
              (else
                (set `self.WeaponType` 0)
                (set `self.AmmoCount` 100)
                (goto _label_8))))
          (:`2`
            (`|SpawnActorFromClass` "/Game/Blueprints/GAB_SpaceShooterPlayerProj03.GAB_SpaceShooterPlayerProj03_C" (`self.GetTransform`) "AdjustIfPossibleButDontSpawnIfColliding" "OverrideRootScale" null null)
            (`GameplayStatics.PlaySoundAtLocation` "/Game/ImportedSounds/discord-notification.discord-notification" (0.0 0.0 0.0) (struct) 1.0 1.0 0.0 null null null)
            (`KismetSystemLibrary.Delay` 0.15)
            (set `self.AmmoCount` (- (`self.AmmoCount`) 2))
            (if (> (`self.AmmoCount`) 0)
              (goto _label_8)
              (else
                (set `self.WeaponType` 0)
                (set `self.AmmoCount` 100)
                (goto _label_8))))
          (:`3`
            (`|SpawnActorFromClass` "/Game/Blueprints/GAB_SpaceShooterPlayerProj04.GAB_SpaceShooterPlayerProj04_C" (`self.GetTransform`) "AdjustIfPossibleButDontSpawnIfColliding" "OverrideRootScale" null null)
            (`GameplayStatics.PlaySoundAtLocation` "/Game/ImportedSounds/quack.quack" (0.0 0.0 0.0) (struct) 1.0 1.0 0.0 null null null)
            (`KismetSystemLibrary.Delay` 0.05)
            (set `self.AmmoCount` (- (`self.AmmoCount`) 1))
            (if (> (`self.AmmoCount`) 0)
              (goto _label_8)
              (else
                (set `self.WeaponType` 0)
                (set `self.AmmoCount` 100)
                (goto _label_8))))))))
  (:`Released`
    (set `self.Firing` false)))

(fn `Get Player Health`
  (returns (`Player Health` :type Integer))
  (return (`self.Health`)))

(fn `Get Score`
  (returns (Score :type Integer))
  (return 0))

(fn `GetAmmoCount`
  (returns (AmmoCount :type Integer))
  (return (`self.AmmoCount`)))

(fn `GetWeaponTYpe`
  (returns (WeaponType :type Integer))
  (return (`self.WeaponType`)))

(fn `UserConstructionScript`)